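; BP_TileMapActor is a tile map segment that populates itself with rodents and triggers generation of the next segment as the player crosses it.
; On BeginPlay it spawns a row of BP_Rodent actors along X from the PaperTileMap's location, with randomly scaled spacing.
; BP_PixelCharacter overlapping Box_MapStart arms a flag, so a later overlap with Box_MapEnd calls GenerateNextTileMap on the spawner, guarded by DoOnce.
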(event OnComponentBeginOverlap(Box_MapEnd)
  (params (OverlappedComponent :type Primitive%20Component%20Object%20Reference) (OtherActor :type Actor%20Object%20Reference) (OtherComp :type Primitive%20Component%20Object%20Reference) (OtherBodyIndex :type Integer) (bFromSweep :type Boolean) (SweepResult :type Hit%20Result%20Structure%20%28by%20ref%29))
  (Utilities|Casting|CastToBP_PixelCharacter OtherActor)
  (if (Variables|Default|GetIsMapStartStepped)
    (Utilities|FlowControl|DoOnce false
      (:Completed
        (Default|GenerateNextTileMap (Variables|Default|GetBP_TileMapSpawner))))))

(event OnComponentBeginOverlap(Box_MapStart)
  (params (OverlappedComponent :type Primitive%20Component%20Object%20Reference) (OtherActor :type Actor%20Object%20Reference) (OtherComp :type Primitive%20Component%20Object%20Reference) (OtherBodyIndex :type Integer) (bFromSweep :type Boolean) (SweepResult :type Hit%20Result%20Structure%20%28by%20ref%29))
  (Utilities|Casting|CastToBP_PixelCharacter OtherActor)
  (Variables|Default|SetIsMapStartStepped true))

(event EventBeginPlay
  (bind _self self)
  (bind _papertilemap (Variables|Default|GetPaperTileMap _self))
  (bind _returnvalue (Transformation|GetWorldLocation _papertilemap))
  (for _index (range 0 18)
    (Game|SpawnActorfromClass "/Game/Pixel2D/Blueprints/Enemy/SimpleAI/BP_Rodent.BP_Rodent_C" (Math|Transform|MakeTransform (Math|Vector|MakeVector (+ (* _index (Math|Random|RandomFloatinRange 3e+01 5e+01)) (.x _returnvalue)) (.y _returnvalue) (.z _returnvalue)) (Math|Rotator|MakeRotator 0.0 0.0 -1.8e+02) "1,1,1") "Undefined" 0 0)))

(event Collision|EventActorBeginOverlap
  (params (OtherActor :type Actor%20Object%20Reference)))

(event EventTick
  (params (DeltaSeconds :type Float%20%28single-precision%29)))

(fn ConstructionScript)