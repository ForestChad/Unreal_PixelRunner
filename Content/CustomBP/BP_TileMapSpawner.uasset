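; Spawner actor that lays out 2D Paper tile map segments in sequence along the X axis.
; Each spawn creates a BP_TileMapActor holding a reference back to the spawner, assigns it the next entry from a TileMaps array and advances the X offset by a fixed step.
; The array index wraps to repeat the maps endlessly.
; The first segment spawns on BeginPlay and later ones on GenerateNextTileMap calls.
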(event Custom|GenerateNextTileMap
  (CallFunction|SpawnandSetTileMap))

(event Custom|SpawnAndSetTileMap
  (bind _returnvalue (Game|SpawnActorfromClass "/Game/CustomBP/BP_TileMapActor.BP_TileMapActor_C" (Math|Transform|MakeTransform (Math|Vector|MakeVector (Variables|Default|GetTileMapOffsetX) 0.0 0.0) "0, 0, 0" "1,1,1") "Undefined" 0 self 0))
  (Class|PaperTileMapComponent|SetTileMap (Variables|/Game/CustomBP/BP_TileMapActor.BP_TileMapActor_C|GetPaperTileMap _returnvalue) (Utilities|Array|Get(acopy) (Variables|Default|GetTileMaps) (Variables|Default|GetIndexOfMapToGenerateNext)))
  (Variables|Default|SetTileMapOffsetX (+ (Variables|Default|GetTileMapOffsetX) 1e+03))
  (Variables|Default|SetIndexOfMapToGenerateNext (+ (Variables|Default|GetIndexOfMapToGenerateNext) 1))
  (if (== (Variables|Default|GetIndexOfMapToGenerateNext) (Utilities|Array|Length (Variables|Default|GetTileMaps)))
    (Variables|Default|SetIndexOfMapToGenerateNext 0)))

(event EventBeginPlay
  (CallFunction|SpawnandSetTileMap))

(event Collision|EventActorBeginOverlap
  (params (OtherActor :type Actor%20Object%20Reference)))

(event EventTick
  (params (DeltaSeconds :type Float%20%28single-precision%29)))

(fn ConstructionScript)